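; BP_WaterLevel is a water hazard that drowns the player's skull rabbit pawn on contact.
; It plays a river rushing sound at its location on BeginPlay.
; When a PAWN_SkullRabbit's box component enters WaterLevelBoundingBox, it sets IsDrowning in player 0's BP_HopperController AnimPack and calls Die on that controller.
; It then plays the drowning sound at the water actor's own location.
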(event `self.ReceiveBeginPlay`
  (`GameplayStatics.PlaySoundAtLocation` "/Game/Sounds/A_River_rushing_SFX_Cue.A_River_rushing_SFX_Cue" (`self.K2_GetActorLocation`) (struct) 1.0 1.0 0.0 null null null))

(event `self.WaterLevelBoundingBox.OnComponentBeginOverlap`
  (params (OverlappedComponent :type "PrimitiveComponent Object Reference") (OtherActor :type "Actor Object Reference") (OtherComp :type "PrimitiveComponent Object Reference") (OtherBodyIndex :type Integer) (bFromSweep :type Boolean) (SweepResult :type "HitResult Structure (by ref)"))
  (cast `/Game/BluePrints/SkullRabbit/PAWN_SkullRabbit` OtherActor)
  (cast `BoxComponent` OtherComp)
  (bind _asbp_hopper_controller (cast `/Game/BluePrints/BP_HopperController` (`GameplayStatics.GetPlayerController` 0)))
  (setmembers `/Game/BluePrints/SkullRabbit/S_AnimPack` :`StructRef` (`/Game/BluePrints/BP_HopperController.animPack` _asbp_hopper_controller) :`isDrowning` true)
  (`/Game/BluePrints/BP_HopperController.Die` _asbp_hopper_controller)
  (`GameplayStatics.PlaySoundAtLocation` "/Game/Sounds/A_Drowning_SFX_Cue.A_Drowning_SFX_Cue" (`self.K2_GetActorLocation`) (struct) 1.0 1.0 0.0 null null null))

(fn `UserConstructionScript`)