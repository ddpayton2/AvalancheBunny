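; BP_Block is a falling-block hazard that can crush the SkullRabbit pawn, with a uniform Scale applied at construction.
; When Cube hits anything other than the rabbit, it stops simulating physics and plays a world camera shake and thump.
; A rabbit overlap while the Bottom component has nonzero velocity calls Die on BP_HopperController.
; The crunch sound mistakenly uses that velocity vector as its location.
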(event `self.Cube.OnComponentHit`
  (params (HitComponent :type "PrimitiveComponent Object Reference") (OtherActor :type "Actor Object Reference") (OtherComp :type "PrimitiveComponent Object Reference") (NormalImpulse :type "Vector Structure") (Hit :type "HitResult Structure (by ref)"))
  (bind _returnvalue (`SceneComponent.K2_GetComponentLocation` (`self.Cube`)))
  (cast `/Game/BluePrints/SkullRabbit/PAWN_SkullRabbit` OtherActor
    (:`CastFailed`
      (`PrimitiveComponent.SetSimulatePhysics` (`self.Cube`) false)
      (`GameplayStatics.PlayWorldCameraShake` "/Game/BluePrints/BP_ScreenShake.BP_ScreenShake_C" _returnvalue 0.0 1500.0)
      (`GameplayStatics.PlaySoundAtLocation` "/Game/Sounds/A_Rock_Thump_SFX_Cue.A_Rock_Thump_SFX_Cue" _returnvalue (struct) 1.0 1.0 0.0 null null null))))

(event `self.ReceiveActorBeginOverlap`
  (params (OtherActor :type "Actor Object Reference"))
  (cast `/Game/BluePrints/SkullRabbit/PAWN_SkullRabbit` OtherActor)
  (bind _returnvalue (`PrimitiveComponent.GetPhysicsLinearVelocity` (`self.Bottom`) "None"))
  (if (not (== _returnvalue (0.0 0.0 0.0)))
    (`GameplayStatics.PlaySoundAtLocation` "/Game/Sounds/A_Crunching_Cue.A_Crunching_Cue" _returnvalue (struct) 1.0 1.0 0.0 null null null)
    (bind _asbp_hopper_controller (cast `/Game/BluePrints/BP_HopperController` (`GameplayStatics.GetPlayerController` 0)))
    (`/Game/BluePrints/BP_HopperController.Die` _asbp_hopper_controller)))

(event `self.ReceiveBeginPlay`)

(fn `UserConstructionScript`
  (bind _scale (`self.Scale`))
  (`self.SetActorScale3D` (`KismetMathLibrary.MakeVector` _scale _scale _scale)))