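; Block spawner for the avalanche game mode that drops BP_Block actors at random points inside its BoundingBox.
; On BeginPlay it checks the game mode's FranticModeIsOn flag to choose normal or frantic spawning.
; Normal spawning creates random-sized batches of large blocks, while frantic spawning creates single tiny blocks far more often.
; Both spawn functions set looping timers by function name, and the construction script also calls SpawnBlocks.
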(event `self.ReceiveBeginPlay`
  (bind _asbp_avalanche_game_mode (cast `/Game/BluePrints/BP_AvalancheGameMode` (`GameplayStatics.GetGameMode`)))
  (if (`/Game/BluePrints/BP_AvalancheGameMode.FranticModeIsOn` _asbp_avalanche_game_mode)
    (`self.SpawnBlocksFrantic`)
    (else
      (`self.SpawnBlocks`))))

(fn `SpawnBlocks`
  (bind _boundingbox (`self.BoundingBox`))
  ;[1 1 1] Time
  (`KismetSystemLibrary.K2_SetTimer` null "SpawnBlocks" 0.6 true)
  (for _ (range (+ (`KismetMathLibrary.RandomInteger` 10) 1))
    (`|SpawnActorFromClass` "/Game/BluePrints/BP_Block.BP_Block_C" (`KismetMathLibrary.Conv_VectorToTransform` (`KismetMathLibrary.RandomPointInBoundingBox` (`SceneComponent.K2_GetComponentLocation` _boundingbox) (`BoxComponent.BoxExtent` _boundingbox))) "AdjustIfPossibleButDontSpawnIfColliding" "OverrideRootScale" null (`KismetMathLibrary.RandomFloatInRange` 2.0 4.0) null)))

(fn `SpawnBlocksFrantic`
  (bind _boundingbox (`self.BoundingBox`))
  (`KismetSystemLibrary.K2_SetTimer` null "Spawn Blocks Frantic" 0.1 true)
  (`|SpawnActorFromClass` "/Game/BluePrints/BP_Block.BP_Block_C" (`KismetMathLibrary.Conv_VectorToTransform` (`KismetMathLibrary.RandomPointInBoundingBox` (`SceneComponent.K2_GetComponentLocation` _boundingbox) (`BoxComponent.BoxExtent` _boundingbox))) "AdjustIfPossibleButDontSpawnIfColliding" "OverrideRootScale" null (`KismetMathLibrary.RandomFloatInRange` 0.1 0.25) null))

(fn `UserConstructionScript`
  (switch `int` 0
    (:`Default`
      (`self.SpawnBlocks`))))