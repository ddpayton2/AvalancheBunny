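; Player controller for the skull rabbit in the Avalanche game mode, handling movement, jumping, death and winning.
; Jump input launches from the ground or traces forward to bounce off walls, with short movement stuns; a similar trace drives ledge climbing.
; An AnimPack struct holds jump and animation state, while Tick refills jumps when grounded and updates the game mode score.
; Die ragdolls the mesh, and both Die and Win lock input and show end screens.
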(event `self.ReceiveBeginPlay`
  (bind _ascharacter (cast `Character` (`self.K2_GetPawn`)))
  (set `self.controlledCharacter` _ascharacter)
  (bind _asbp_avalanche_game_mode (cast `/Game/BluePrints/BP_AvalancheGameMode` (`GameplayStatics.GetGameMode`)))
  (set `self.gameMode` _asbp_avalanche_game_mode))

(event `self.ReceiveTick`
  (params (DeltaSeconds :type "Float (single-precision)"))
  (`self.checkIfFalling`)
  (`self.tryFollowRagdoll`)
  (`/Game/BluePrints/BP_AvalancheGameMode.AdjustScore` (`self.gameMode`)))

(event `InputAxis|MoveForward`
  (params (AxisValue :type "Float (single-precision)"))
  (if (not (`self.movementLocked`))
    (`Pawn.AddMovementInput` (`self.K2_GetPawn`) (`KismetMathLibrary.GetForwardVector` (`KismetMathLibrary.MakeRotator` 0.0 0.0 (.yaw (`self.GetControlRotation`)))) AxisValue false)))

(event `InputAxis|MoveRight`
  (params (AxisValue :type "Float (single-precision)"))
  (if (not (`self.movementLocked`))
    (`Pawn.AddMovementInput` (`self.K2_GetPawn`) (`KismetMathLibrary.GetRightVector` (`KismetMathLibrary.MakeRotator` 0.0 0.0 (.yaw (`self.GetControlRotation`)))) AxisValue false)))

(event `InputAxis|Turn`
  (params (AxisValue :type "Float (single-precision)"))
  (if (not (`self.movementLocked`))
    (`Pawn.AddControllerYawInput` (`self.K2_GetPawn`) AxisValue)))

(event `InputAxis|LookUp`
  (params (AxisValue :type "Float (single-precision)"))
  (if (not (`self.movementLocked`))
    (`Pawn.AddControllerPitchInput` (`self.K2_GetPawn`) AxisValue)))

(event `InputAction|Jump`
  (params (Key :type "Key Structure"))
  (bind (_maxjumps _jumpsleft) (break `/Game/BluePrints/SkullRabbit/S_AnimPack` (`self.animPack`)))
  (:`Pressed`
    (if (`NavMovementComponent.IsFalling` (`Character.CharacterMovement` (`self.controlledCharacter`)))
      (`self.tryWallJump`)
      (`KismetSystemLibrary.Delay` 1.5 :!label _label)
      (set `self.canWallJump` true)
      (elif (> _jumpsleft 0)
        (`Character.LaunchCharacter` (`self.controlledCharacter`) (0.0 0.0 750.0) false false)
        (`KismetSystemLibrary.Delay` 0.05)
        (bind _result (`/Engine/EditorBlueprintResources/StandardMacros.DecrementInt` _jumpsleft)
          (:`  `
            (setmembers `/Game/BluePrints/SkullRabbit/S_AnimPack` :`StructRef` (`self.animPack`) :`jumpsLeft` _result)
            (`GameplayStatics.PlaySoundAtLocation` "/Game/Sounds/A_Jumping_Cue.A_Jumping_Cue" (`self.K2_GetActorLocation`) (struct) 1.0 1.0 0.0 null null null)
            (goto _label)))))))

(event `applyMovementStun`
  (params (time :type "Float (double-precision)"))
  (set `self.movementLocked` true)
  (`KismetSystemLibrary.Delay` time)
  (set `self.movementLocked` false)
  (setmembers `/Game/BluePrints/SkullRabbit/S_AnimPack` :`StructRef` (`self.animPack`) :`isWallJumping` false :`isClimbingLedge` false))

(event `InputAction|Kill Self`
  (params (Key :type "Key Structure"))
  (:`Pressed`
    (`self.Die`)))

(event `Die`
  (bind _animpack (`self.animPack`))
  (bind _mesh (`Character.Mesh` (`self.controlledCharacter`)))
  (bind _mesh_2 (`Character.Mesh` (`self.controlledCharacter`)))
  (if (`.isDrowning_21_83D41C73453EB01CD26957ACB7CCC148` (break `/Game/BluePrints/SkullRabbit/S_AnimPack` _animpack))
    (`self.DisableInput` self)
    (`WidgetLayoutLibrary.RemoveAllWidgets`)
    (bind _returnvalue (`|CreateWidget` "/Game/BluePrints/WBP_DeathScreen.WBP_DeathScreen_C"))
    (`UserWidget.AddToViewport` _returnvalue 0)
    (set `PlayerController.bShowMouseCursor` true (`GameplayStatics.GetPlayerController` 0))
    (`KismetSystemLibrary.Delay` 3.0)
    (`PrimitiveComponent.SetCollisionEnabled` _mesh "PhysicsOnly")
    (`PrimitiveComponent.SetSimulatePhysics` _mesh true)
    (else
      (setmembers `/Game/BluePrints/SkullRabbit/S_AnimPack` :`StructRef` _animpack :`isCrushed` true)
      (`PrimitiveComponent.SetCollisionEnabled` _mesh_2 "PhysicsOnly")
      (`PrimitiveComponent.SetSimulatePhysics` _mesh_2 true)
      (`self.DisableInput` self)
      (`WidgetLayoutLibrary.RemoveAllWidgets`)
      (bind _returnvalue_2 (`|CreateWidget` "/Game/BluePrints/WBP_DeathScreen.WBP_DeathScreen_C"))
      (`UserWidget.AddToViewport` _returnvalue_2 0)
      (set `PlayerController.bShowMouseCursor` true (`GameplayStatics.GetPlayerController` 0)))))

(event `Win`
  (if (not (`self.hasWon`))
    (set `self.hasWon` true)
    (`self.DisableInput` self)
    (`WidgetLayoutLibrary.RemoveAllWidgets`)
    (bind _returnvalue (`|CreateWidget` "/Game/BluePrints/WBP_WinScreen.WBP_WinScreen_C"))
    (`UserWidget.AddToViewport` _returnvalue 0)
    (set `PlayerController.bShowMouseCursor` true (`GameplayStatics.GetPlayerController` 0))))

(fn `checkIfFalling`
  (bind _animpack (`self.animPack`))
  (if (not (`NavMovementComponent.IsFalling` (`Character.CharacterMovement` (`self.controlledCharacter`))))
    (setmembers `/Game/BluePrints/SkullRabbit/S_AnimPack` :`StructRef` _animpack :`jumpsLeft` (`.maxJumps_9_B5EB861944100FAC0EC96CA169EA9C9D` (break `/Game/BluePrints/SkullRabbit/S_AnimPack` _animpack)) :`isWallJumping` false :`isClimbingLedge` false)))

(fn `tryClimbLedge`
  (if (not (`.isDrowning_21_83D41C73453EB01CD26957ACB7CCC148` (break `/Game/BluePrints/SkullRabbit/S_AnimPack` (`self.animPack`))))
    (bind _aspawn_skull_rabbit (cast `/Game/BluePrints/SkullRabbit/PAWN_SkullRabbit` (`self.controlledCharacter`)))
    (bind _arrow1 (`/Game/BluePrints/SkullRabbit/PAWN_SkullRabbit.Arrow1` _aspawn_skull_rabbit))
    (bind _returnvalue (`SceneComponent.K2_GetComponentLocation` _arrow1))
    (bind _returnvalue_2 (* (`SceneComponent.GetForwardVector` _arrow1) 100.0))
    (bind (_outhit _returnvalue_3) (`KismetSystemLibrary.LineTraceSingle` _returnvalue (+ _returnvalue _returnvalue_2) "TraceTypeQuery1"))
    (if (not _returnvalue_3)
      (setmembers `/Game/BluePrints/SkullRabbit/S_AnimPack` :`StructRef` (`self.animPack`) :`isClimbingLedge` true)
      (set `MovementComponent.Velocity` (+ _returnvalue_2 (0.0 0.0 500.0)) (`Character.CharacterMovement` (`self.controlledCharacter`)))
      (`self.applyMovementStun` 0.3))))

(fn `tryFollowRagdoll`)

(fn `tryWallJump`
  (bind _controlledcharacter (`self.controlledCharacter`))
  (if (`self.canWallJump`)
    (bind _aspawn_skull_rabbit (cast `/Game/BluePrints/SkullRabbit/PAWN_SkullRabbit` (`self.controlledCharacter`)))
    (bind _arrow1 (`/Game/BluePrints/SkullRabbit/PAWN_SkullRabbit.Arrow1` _aspawn_skull_rabbit))
    (bind _returnvalue (`SceneComponent.K2_GetComponentLocation` _arrow1))
    (bind _returnvalue_2 (* (`SceneComponent.GetForwardVector` _arrow1) 100.0))
    (bind (_outhit _returnvalue_3) (`KismetSystemLibrary.LineTraceSingle` _returnvalue (+ _returnvalue _returnvalue_2) "TraceTypeQuery1"))
    (if _returnvalue_3
      (bind _output_get (set `MovementComponent.Velocity` (+ (* (`KismetMathLibrary.Normal` (`KismetMathLibrary.MirrorVectorByNormal` _returnvalue_2 (`.ImpactNormal` (`GameplayStatics.BreakHitResult` _outhit)))) 400.0) (0.0 0.0 600.0)) (`Character.CharacterMovement` _controlledcharacter)))
      (`self.K2_SetActorRotation` _controlledcharacter (`KismetMathLibrary.MakeRotator` 0.0 0.0 (.yaw (`KismetMathLibrary.MakeRotFromXY` _output_get _output_get))) false)
      (setmembers `/Game/BluePrints/SkullRabbit/S_AnimPack` :`StructRef` (`self.animPack`) :`isWallJumping` true)
      (`self.applyMovementStun` 0.3)
      (set `self.canWallJump` false))))

(fn `UserConstructionScript`)